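; BP_InfectingNPC is an NPC that the player rat can bite, becoming infected on the second bite.
; Its InfectionRange overlaps toggle the rat's in-bite-range flag, and entering also hands the rat a reference to this NPC.
; The Bite event records the first bite, then destroys the actor on the second, playing a scream and clearing its can-bite flag each time.
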(event OnComponentBeginOverlap(InfectionRange)
  (params (OverlappedComponent :type Primitive%20Component%20Object%20Reference) (OtherActor :type Actor%20Object%20Reference) (OtherComp :type Primitive%20Component%20Object%20Reference) (OtherBodyIndex :type Integer) (bFromSweep :type Boolean) (SweepResult :type Hit%20Result%20Structure%20%28by%20ref%29))
  (bind _asbp_player_rat (Utilities|Casting|CastToBP_PlayerRat OtherActor))
  (Variables|/Game/PlayerCharacter/BP_PlayerRat.BP_PlayerRat_C|SetB_InBiteRange _asbp_player_rat true)
  (Variables|/Game/PlayerCharacter/BP_PlayerRat.BP_PlayerRat_C|SetInfected%20NPC%20Reference _asbp_player_rat self))

(event OnComponentEndOverlap(InfectionRange)
  (params (OverlappedComponent :type Primitive%20Component%20Object%20Reference) (OtherActor :type Actor%20Object%20Reference) (OtherComp :type Primitive%20Component%20Object%20Reference) (OtherBodyIndex :type Integer))
  (bind _asbp_player_rat (Utilities|Casting|CastToBP_PlayerRat OtherActor))
  (Variables|Default|SetAs%20BP%20Player%20Rat _asbp_player_rat)
  (Variables|/Game/PlayerCharacter/BP_PlayerRat.BP_PlayerRat_C|SetB_InBiteRange _asbp_player_rat false))

(event EventBite
  (params (Bite :type Boolean))
  (if Bite
    (if (Variables|Default|GetB_Is%20Bitten)
      (Variables|Default|SetB_Is%20Bitten%20Twice true)
      (Development|PrintString "Infected")
      (Audio|PlaySound2D "/Game/Audio/SE/Bite_Scream_1_Cue.Bite_Scream_1_Cue" 1.0 1.0 0.0 0 0)
      (Variables|Default|SetB_CanIBite false)
      (Actor|DestroyActor)
      (else
        (Variables|Default|SetB_Is%20Bitten true)
        (Development|PrintString "First bite")
        (Audio|PlaySound2D "/Game/Audio/SE/Bite_Scream_1_Cue.Bite_Scream_1_Cue" 1.0 1.0 0.0 0 0)
        (Variables|Default|SetB_CanIBite false)))))

(fn ConstructionScript)