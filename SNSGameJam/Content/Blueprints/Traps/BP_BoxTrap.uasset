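; BP_BoxTrap is a trap actor that drops a propped-up box when the player rat enters its trigger.
; The Box component's overlap casts to BP_PlayerRat and fires once, hiding the Cylinder and disabling its collision.
; The BoxFall timeline then lerps the static mesh's relative rotation and location from tilted and raised to level and lowered.
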(event OnComponentBeginOverlap(Box)
  (params (OverlappedComponent :type Primitive%20Component%20Object%20Reference) (OtherActor :type Actor%20Object%20Reference) (OtherComp :type Primitive%20Component%20Object%20Reference) (OtherBodyIndex :type Integer) (bFromSweep :type Boolean) (SweepResult :type Hit%20Result%20Structure%20%28by%20ref%29))
  (bind _cylinder (Variables|Default|GetCylinder))
  (Utilities|Casting|CastToBP_PlayerRat OtherActor)
  (Utilities|FlowControl|DoOnce false
    (:Completed
      (Rendering|SetVisibility _cylinder false false)
      (Collision|SetCollisionEnabled _cylinder "NoCollision")
      (bind _newtrack_0 (Timeline|BoxFall PlayFromStart)
        (:Update
          (Transformation|SetRelativeRotation (Variables|Default|GetStaticMesh) (Math|Rotator|MakeRotator -1.8e+02 (Math|Float|Lerp 3e+01 0.0 _newtrack_0) 9e+01) false false)
          (Transformation|SetRelativeLocation (Variables|Default|GetStaticMesh) (Math|Vector|MakeVector 0.0 (Math|Float|Lerp -5e+01 -2e+01 _newtrack_0) (Math|Float|Lerp 75.0 25.0 _newtrack_0)) false false))))))

(event EventBeginPlay)

(event Collision|EventActorBeginOverlap
  (params (OtherActor :type Actor%20Object%20Reference)))

(event EventTick
  (params (DeltaSeconds :type Float%20%28single-precision%29)))

(fn ConstructionScript)