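; Behavior tree task that advances an NPC's patrol point index along its patrol path.
; On AI execute, it casts the controlled pawn to BP_Human and reads the length of that human's PatrolPath points.
; If the next index is within range, it writes it to the BBPathIndex blackboard key and finishes successfully.
; At the last point or on a failed cast, the index stays unchanged and the task never calls FinishExecute.
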(event EventReceiveExecuteAI
  (params (OwnerController :type AI%20Controller%20Object%20Reference) (ControlledPawn :type Pawn%20Object%20Reference))
  (bind _bb_pathindex (Variables|Default|GetBB_PathIndex))
  (bind _returnvalue (Class|BTFunctionLibrary|GetBlackboardValueasInt _bb_pathindex))
  (bind _returnvalue_2 (+ _returnvalue 1))
  (bind _asbp_human (Utilities|Casting|CastToBP_Human ControlledPawn))
  (if (<= _returnvalue_2 (- (Utilities|Array|Length (Variables|/Game/AI/NPC/BP_PatrolPath.BP_PatrolPath_C|GetPath%20Points (Variables|/Game/AI/NPC/BP_Human.BP_Human_C|GetPatrolPath _asbp_human))) 1))
    (Class|BTFunctionLibrary|SetBlackboardValueasInt (Variables|Default|GetBB_PathIndex) _returnvalue_2)
    (AI|BehaviorTree|FinishExecute true)))