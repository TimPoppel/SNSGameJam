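; BP_Human is a human NPC that the player rat can bite and infect, and that kills the rat on contact with its box.
; An infection sphere overlap flags the rat as in bite range, and interact-range events show a screen-space "Bite" widget.
; A first bite attaches infection particles; a second destroys the human, updating RatMode_GM's alive count and chase list, while SuperBit infects instantly.
; Construction randomizes body color.
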(event OnComponentBeginOverlap(InfectionRange)
  (params (OverlappedComponent :type Primitive%20Component%20Object%20Reference) (OtherActor :type Actor%20Object%20Reference) (OtherComp :type Primitive%20Component%20Object%20Reference) (OtherBodyIndex :type Integer) (bFromSweep :type Boolean) (SweepResult :type Hit%20Result%20Structure%20%28by%20ref%29))
  (bind _asbp_player_rat (Utilities|Casting|CastToBP_PlayerRat OtherActor))
  (Variables|/Game/PlayerCharacter/BP_PlayerRat.BP_PlayerRat_C|SetB_InBiteRange _asbp_player_rat true)
  (Variables|/Game/PlayerCharacter/BP_PlayerRat.BP_PlayerRat_C|SetBP_Human_Reference _asbp_player_rat self))

(event OnComponentEndOverlap(InfectionRange)
  (params (OverlappedComponent :type Primitive%20Component%20Object%20Reference) (OtherActor :type Actor%20Object%20Reference) (OtherComp :type Primitive%20Component%20Object%20Reference) (OtherBodyIndex :type Integer))
  (bind _asbp_player_rat (Utilities|Casting|CastToBP_PlayerRat OtherActor))
  (Variables|Default|SetAs%20BP%20Player%20Rat _asbp_player_rat)
  (Variables|/Game/PlayerCharacter/BP_PlayerRat.BP_PlayerRat_C|SetB_InBiteRange _asbp_player_rat false))

(event OnComponentBeginOverlap(Box)
  (params (OverlappedComponent :type Primitive%20Component%20Object%20Reference) (OtherActor :type Actor%20Object%20Reference) (OtherComp :type Primitive%20Component%20Object%20Reference) (OtherBodyIndex :type Integer) (bFromSweep :type Boolean) (SweepResult :type Hit%20Result%20Structure%20%28by%20ref%29))
  ;[1 1 1] Killing Rats
  (if (== OtherActor (Game|GetPlayerCharacter 0))
    (bind _asbp_player_rat (Utilities|Casting|CastToBP_PlayerRat OtherActor))
    (Default|DeathState _asbp_player_rat)
    (Actor|DestroyActor _asbp_player_rat)))

(event EventOnInteractOutRange
  (bind _interactwidgetcomp (Variables|Default|GetInteractWidgetComp)
    (:then
      (Components|DestroyComponent _interactwidgetcomp))
    (:else)))

(event EventOnInteractRange
  (params (Rat :type BP%20Player%20Rat%20Object%20Reference))
  (Variables|Default|GetInteractWidgetComp
    (:then)
    (:else
      (bind _asplayer_controller (Utilities|Casting|CastToPlayerController (Pawn|GetController Rat)))
      (bind _returnvalue (UserInterface|CreateWidget "/Game/Menu/WBP_Interaction.WBP_Interaction_C" _asplayer_controller "Bite"))
      (bind _returnvalue_2 (AddComponent|AddWidgetComponent false (Math|Transform|MakeTransform "0, 0,-80.000000" "0, 0, 0" "1,1,1")))
      (bind _output_get (Variables|Default|SetInteractWidgetComp _returnvalue_2))
      (UserInterface|SetWidget _output_get _returnvalue)
      (Class|WidgetComponent|SetWidgetSpace _output_get "Screen")
      (Class|WidgetComponent|SetDrawatDesiredSize _output_get true)
      (Collision|SetCollisionEnabled _output_get "NoCollision"))))

(event EventSuperBit
  (Variables|Default|SetB_Is%20Bitten%20Twice true)
  (Development|PrintString "Infected")
  (Audio|PlaySound2D "/Game/Audio/SE/Bite_Scream_1_Cue.Bite_Scream_1_Cue" 1.0 1.0 0.0 0 0)
  (Variables|Default|SetB_CanIBite false)
  (Actor|DestroyActor))

(event EventBeginPlay
  ;[1 1 1] humans alive
  (bind _asrat_mode_gm (Utilities|Casting|CastToRatMode_GM (Game|GetGameMode)))
  (Variables|/Game/RatMode_GM.RatMode_GM_C|SetHumansAlive _asrat_mode_gm (+ (Variables|/Game/RatMode_GM.RatMode_GM_C|GetHumansAlive _asrat_mode_gm) 1)))

(event EventBite
  (params (Bite :type Boolean))
  (if Bite
    (if (Variables|Default|GetB_Is%20Bitten)
      (Variables|Default|SetB_Is%20Bitten%20Twice true)
      (Development|PrintString "Infected")
      (Audio|PlaySound2D "/Game/Audio/SE/Bite_Scream_1_Cue.Bite_Scream_1_Cue" 1.0 1.0 0.0 0 0)
      (Variables|Default|SetB_CanIBite false)
      ;[1 1 1] humans alive
      (bind _asrat_mode_gm (Utilities|Casting|CastToRatMode_GM (Game|GetGameMode)))
      (Variables|/Game/RatMode_GM.RatMode_GM_C|SetHumansAlive _asrat_mode_gm (- (Variables|/Game/RatMode_GM.RatMode_GM_C|GetHumansAlive _asrat_mode_gm) 1))
      (bind _asrat_mode_gm_2 (Utilities|Casting|CastToRatMode_GM (Game|GetGameMode)))
      (Utilities|Array|RemoveItem (Variables|/Game/RatMode_GM.RatMode_GM_C|GetChasers _asrat_mode_gm_2) self)
      (Default|EndChase _asrat_mode_gm_2)
      (Actor|DestroyActor)
      (else
        (Variables|Default|SetB_Is%20Bitten true)
        (Development|PrintString "First bite")
        (Audio|PlaySound2D "/Game/Audio/SE/Bite_Scream_1_Cue.Bite_Scream_1_Cue" 1.0 1.0 0.0 0 0)
        (Variables|Default|SetB_CanIBite false)
        (bind _returnvalue (Effects|SpawnEmitterAttached "/Game/VisualEffects/PS_Infected.PS_Infected" (Variables|Character|GetMesh) "None" "0, 0,130.000000"))
        (Variables|Default|SetParticle%20REF _returnvalue)))))

(fn ConstructionScript
  (bind _returnvalue (Rendering|Material|CreateDynamicMaterialInstance (Variables|Character|GetMesh) 0 0 "None" :!class /Script/Engine.PrimitiveComponent))
  (Rendering|Material|SetVectorParameterValue _returnvalue "BodyColor" (Math|Color|MakeColor (Math|Random|RandomFloat) (Math|Random|RandomFloat) (Math|Random|RandomFloat)) :!class /Script/Engine.MaterialInstanceDynamic))