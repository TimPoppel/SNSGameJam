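; Behavior Tree task that supplies the next patrol destination for a BP_Human NPC and takes it out of any chase.
; It reads the patrol path point at the blackboard index, converts it to world space and writes it to the path vector key.
; It then removes the human from the RatMode_GM Chasers list, calls EndChase and finishes successfully.
; Without a valid patrol path or successful casts, the task never calls FinishExecute.
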(event EventReceiveExecuteAI
  (params (OwnerController :type AI%20Controller%20Object%20Reference) (ControlledPawn :type Pawn%20Object%20Reference))
  (bind _asbp_human (Utilities|Casting|CastToBP_Human ControlledPawn))
  (bind _patrolpath (Variables|/Game/AI/NPC/BP_Human.BP_Human_C|GetPatrolPath _asbp_human)
    (:then
      (AI|BehaviorTree|SetBlackboardValueasVector (Variables|Default|GetBB_PathVector) (Math|Transform|TransformLocation (Transformation|GetActorTransform _patrolpath) (Utilities|Array|Get(acopy) (Variables|/Game/AI/NPC/BP_PatrolPath.BP_PatrolPath_C|GetPath%20Points _patrolpath) (Class|BTFunctionLibrary|GetBlackboardValueasInt (Variables|Default|GetBB_PathIndex)))))
      (bind _asrat_mode_gm (Utilities|Casting|CastToRatMode_GM (Game|GetGameMode)))
      (Utilities|Array|RemoveItem (Variables|/Game/RatMode_GM.RatMode_GM_C|GetChasers _asrat_mode_gm) _asbp_human)
      (Default|EndChase _asrat_mode_gm)
      (AI|BehaviorTree|FinishExecute true))
    (:else)))