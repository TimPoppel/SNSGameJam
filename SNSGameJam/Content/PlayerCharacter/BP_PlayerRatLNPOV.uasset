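; Player rat character for the LN point of view, with axis movement along the capsule's forward and right vectors and jumping.
; On BeginPlay it spawns a separate LNCamera actor as the view target, which interpolates each Tick toward the location of the character's own camera.
; Holding OffsetLeft or OffsetRight shifts the spring arm's target sideways, so the view follows smoothly.
; Turn and LookUp inputs are unwired, leaving no mouse look.
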(event EventBeginPlay
  (Game|SpawnActorfromClass "/Game/PlayerCharacter/LNCamera.LNCamera_C" (Transformation|GetWorldTransform (Variables|Default|GetCamera)) "Undefined" 0 0)
  (bind _outactors (Actor|GetAllActorsOfClass "/Game/PlayerCharacter/LNCamera.LNCamera_C"))
  (Variables|Default|SetLNCameraREF (Utilities|Array|Get(acopy) _outactors))
  (Game|Player|SetViewTargetwithBlend (Game|GetPlayerController 0) (Variables|Default|GetLNCameraREF) 0.0 "VTBlend_Linear" 0.0 false)
  (Transformation|SetActorLocation (Variables|Default|GetLNCameraREF) (Transformation|GetWorldLocation (Variables|Default|GetCamera)) false false))

(event EventTick
  (params (DeltaSeconds :type Float%20%28single-precision%29))
  (Transformation|SetActorLocation (Variables|Default|GetLNCameraREF) (Math|Interpolation|VInterpTo (Transformation|GetActorLocation (Variables|Default|GetLNCameraREF)) (Transformation|GetWorldLocation (Variables|Default|GetCamera)) (Utilities|Time|GetWorldDeltaSeconds) (Variables|Default|GetInterp%20Speed)) false false))

(event Input|ActionEvents|InputActionJump
  (params (Key :type Key%20Structure :default "None"))
  (:Pressed
    (Character|Jump)))

(event Input|ActionEvents|InputActionOffsetLeft
  (params (Key :type Key%20Structure :default "None"))
  (bind _springarm (Variables|Default|GetSpringArm))
  (:Pressed
    (Variables|/Script/Engine.SpringArmComponent|SetTargetOffset _springarm "0,-180.000000, 0"))
  (:Released
    (Variables|/Script/Engine.SpringArmComponent|SetTargetOffset _springarm "0, 0, 0")))

(event Input|ActionEvents|InputActionOffsetRight
  (params (Key :type Key%20Structure :default "None"))
  (bind _springarm (Variables|Default|GetSpringArm))
  (:Pressed
    (Variables|/Script/Engine.SpringArmComponent|SetTargetOffset _springarm "0,180.000000, 0"))
  (:Released
    (Variables|/Script/Engine.SpringArmComponent|SetTargetOffset _springarm "0, 0, 0")))

(event Input|AxisEvents|InputAxisMoveForward
  (params (AxisValue :type Float%20%28single-precision%29))
  (Pawn|Input|AddMovementInput (Math|Vector|GetForwardVector (Variables|Collision|GetCapsuleComponent)) (* AxisValue (Variables|Default|GetMovementMultiplier) (Utilities|Time|GetWorldDeltaSeconds)) false))

(event Input|AxisEvents|InputAxisMoveRight
  (params (AxisValue :type Float%20%28single-precision%29))
  (Pawn|Input|AddMovementInput (Math|Vector|GetRightVector (Variables|Collision|GetCapsuleComponent)) (* AxisValue (Variables|Default|GetMovementMultiplier) (Utilities|Time|GetWorldDeltaSeconds)) false))

(event Input|AxisEvents|InputAxisLookUp
  (params (AxisValue :type Float%20%28single-precision%29)))

(event Input|AxisEvents|InputAxisTurn
  (params (AxisValue :type Float%20%28single-precision%29)))

(fn ConstructionScript)